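; BP_MapChanger is a map exit trigger that saves progress and starts the transition once the map is cleared.
; It spawns a Niagara marker at BeginPlay and reacts when a BP_Vehicle overlaps its sphere while MapCleared is true.
; It records the level as beaten through BP_MPGameInstance, then looks up that level's name in DT_WidgetInfoLoading.
; A found row fills WBP_LoadingScreen; a missing row opens MainMenu.
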(event `self.ReceiveBeginPlay`
  (`NiagaraFunctionLibrary.SpawnSystemAtLocation` "/Game/CyberTanks/MapRelatedBPs/N_Meta.N_Meta" (`SceneComponent.K2_GetComponentLocation` (`self.DefaultSceneRoot`))))

(event `self.Sphere.OnComponentBeginOverlap`
  (params (OverlappedComponent :type "PrimitiveComponent Object Reference") (OtherActor :type "Actor Object Reference") (OtherComp :type "PrimitiveComponent Object Reference") (OtherBodyIndex :type Integer) (bFromSweep :type Boolean) (SweepResult :type "HitResult Structure (by ref)"))
  (`KismetSystemLibrary.IsObjectOfSoftClass` OtherActor "/Game/CyberTanks/TankBase/Vehicle/BP_Vehicle.BP_Vehicle_C"
    (:`True`
      (if (`self.MapCleared`)
        (bind _asbp_mpgame_instance (cast `/Game/CyberTanks/MultiPlayerSetup/BP_MPGameInstance` (`GameplayStatics.GetGameInstance`)))
        (bind _returnvalue (`GameplayStatics.GetCurrentLevelName` true))
        (`/Game/CyberTanks/MultiPlayerSetup/BP_MPGameInstance.ModifySaveFile` :`self` _asbp_mpgame_instance :`BeatenMapName` (`KismetStringLibrary.Conv_StringToName` _returnvalue))
        (bind _returnvalue_2 (`GameplayStatics.GetCurrentLevelName` true))
        (bind _returnvalue_3 (`|GetDataTableRow` "/Game/CyberTanks/UI/LoadingScreens/DT_WidgetInfoLoading.DT_WidgetInfoLoading" (`KismetStringLibrary.Conv_StringToName` _returnvalue_2))
          (:`then`
            (bind (_image _mapname _lore _imagemaybe _drugastrona) (break `/Game/CyberTanks/UI/LoadingScreens/STRUCT_LoadingScreenWidget` _returnvalue_3))
            (bind _returnvalue_4 (`|CreateWidget` "/Game/CyberTanks/UI/LoadingScreens/WBP_LoadingScreen.WBP_LoadingScreen_C" null _image _mapname _lore _imagemaybe _drugastrona))
            (`UserWidget.AddToViewport` _returnvalue_4 0))
          (:`RowNotFound`
            (`GameplayStatics.OpenLevelBySoftObjectPtr` "/Game/CyberTanks/MainMenu/MainMenu.MainMenu")))))))

(fn `UserConstructionScript`)